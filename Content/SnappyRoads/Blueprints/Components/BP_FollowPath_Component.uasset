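; Component that drives its owning actor, apparently a vehicle, continuously along a spline in Snappy Roads.
; On BeginPlay it picks a random start distance away from the spline's end, retrying a few times if a sphere check finds another BP_Vehicle there.
; Each tick advances the distance by speed, wraps it at the spline length and snaps the owner's transform to it, mirroring the distance when Reverse is set.
; Without a valid spline, ticking is disabled.
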(event EventBeginPlay
  (bind _spline (Variables|Core|GetSpline))
  (bind _spline_2 (Variables|Core|GetSpline))
  ;[1 1 1] ValidityCheck
  (Utilities|IsValid _spline_2
    (:Is%20Valid
      (bind _output_get (Variables|Core|SetLength (Spline|GetSplineLength _spline_2)))
      (if (> _output_get 0.0)
        ;[1 1 1] [Move2VehiclesOBP] PlaceRandomlyAlongTheSplineAvoidingOverlaps
        (bind _index (Utilities|FlowControl|ForLoopwithBreak 0 5 :!label _label)
          (:LoopBody
            (bind _output_get_2 (Variables|Core|Set_temp (Math|Random|RandomFloatinRange 0.0 (- _output_get 6e+02))))
            (bind _returnvalue (Collision|SphereOverlapActors (+ (Spline|GetLocationatDistanceAlongSpline _spline _output_get_2 "World") (Math|Vector|RotateVector (Variables|Config|GetOffset) (Spline|GetRotationatDistanceAlongSpline _spline _output_get_2 "World"))) 3e+02 (Utilities|Array|MakeArray "ObjectTypeQuery2") "/Game/SnappyRoads/Blueprints/BP_Vehicle.BP_Vehicle_C"))
            (if (not _returnvalue)
              (goto _label Break)))
          (:Completed
            (Variables|Core|SetCurrentDistance _output_get_2)
            ;[1 1 1] Movement
            (Transformation|SetActorLocationAndRotation (Components|GetOwner) (.location (Spline|GetTransformatDistanceAlongSpline (Variables|Core|GetSpline) (Math|Float|SelectFloat (- (Variables|Core|GetLength) (Variables|Core|GetCurrentDistance)) (Variables|Core|GetCurrentDistance) (Variables|Default|GetReverse)) "World" false)) (.rotation (Spline|GetTransformatDistanceAlongSpline (Variables|Core|GetSpline) (Math|Float|SelectFloat (- (Variables|Core|GetLength) (Variables|Core|GetCurrentDistance)) (Variables|Core|GetCurrentDistance) (Variables|Default|GetReverse)) "World" false)))
            (Variables|Core|SetCurrentDistance (Math|Float|%(Float) (+ (* (stale EventTick DeltaSeconds) (Variables|Config|GetSpeed) 25.0) (Variables|Core|GetCurrentDistance)) (Variables|Core|GetLength)))))
        (else
          (Components|Tick|SetComponentTickEnabled false :!label _label_2))))
    (:Is%20Not%20Valid
      (goto _label_2))))

(event EventTick
  (params (DeltaSeconds :type Float%20%28single-precision%29))
  ;[1 1 1] Movement
  (Transformation|SetActorLocationAndRotation (Components|GetOwner) (.location (Spline|GetTransformatDistanceAlongSpline (Variables|Core|GetSpline) (Math|Float|SelectFloat (- (Variables|Core|GetLength) (Variables|Core|GetCurrentDistance)) (Variables|Core|GetCurrentDistance) (Variables|Default|GetReverse)) "World" false)) (.rotation (Spline|GetTransformatDistanceAlongSpline (Variables|Core|GetSpline) (Math|Float|SelectFloat (- (Variables|Core|GetLength) (Variables|Core|GetCurrentDistance)) (Variables|Core|GetCurrentDistance) (Variables|Default|GetReverse)) "World" false)))
  (Variables|Core|SetCurrentDistance (Math|Float|%(Float) (+ (* DeltaSeconds (Variables|Config|GetSpeed) 25.0) (Variables|Core|GetCurrentDistance)) (Variables|Core|GetLength))))