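; BP_Tunnel is a railway actor that builds a tunnel along the nearest BP_Track at construction time, showing a text component if none is found.
; It projects its location onto the track spline, then lays spline meshes forward or in reverse over a length limited by the track.
; Double tracks use wider meshes centred between rails, and closed loops wrap distances.
; AddPortal caps both ends, optionally adding blocking boxes.
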(event EventBeginPlay)

(event Collision|EventActorBeginOverlap
  (params (OtherActor :type Actor%20Object%20Reference)))

(event EventTick
  (params (DeltaSeconds :type Float%20%28single-precision%29)))

(fn ConstructionScript
  (bind _reverse_tunnel_direction (Variables|Tunnel|GetReverse%20Tunnel%20Direction))
  (bind _reverse_tunnel_direction_2 (Variables|Tunnel|GetReverse%20Tunnel%20Direction))
  (bind _mesh_length (Variables|Default|GetMesh%20Length))
  (bind _defaultsceneroot (Variables|Default|GetDefaultSceneRoot))
  (bind _lenght__m_ (Variables|Tunnel|GetLenght%20%28m%29))
  (bind _defaultsceneroot_2 (Variables|Default|GetDefaultSceneRoot))
  (bind _returnvalue (Transformation|GetWorldLocation _defaultsceneroot))
  (bind _returnvalue_2 (* _lenght__m_ 1e+02))
  (bind _returnvalue_3 (* _returnvalue -1.0))
  (Variables|Tunnel|SetUpdate false)
  ;[1 1 1] Search for BP_Track and create message if search failed
  (Transformation|SetWorldRotation _defaultsceneroot_2 "0, 0, 0" false false)
  (bind (_track_selected _track_pick) (CallFunction|SearchNearestBPTrack (Transformation|GetWorldLocation _defaultsceneroot_2)))
  (bind _output_get (Variables|Default|SetTrackSelected _track_selected))
  (if _output_get
    (Utilities|FlowControl|Sequence
      (:then_0
        ;[1 1 1] Get needed variables from BP_Track
        (bind _output_get_2 (Variables|Default|SetTrack%20Pick _track_pick))
        (bind _output_get_3 (Variables|Default|SetSpline (Variables|/Game/Railway_System/Blueprints/BP_Track.BP_Track_C|GetSpline_Current _output_get_2)))
        (Variables|Default|SetRail%20Top%20Height (Variables|/Game/Railway_System/Blueprints/BP_Track.BP_Track_C|GetRail%20Top%20Height _output_get_2))
        (Variables|Default|SetDoubleTrack (Variables|/Game/Railway_System/Blueprints/BP_Track.BP_Track_C|GetDouble%20Track _output_get_2))
        (Variables|Default|SetClosedLoop (Variables|/Game/Railway_System/Blueprints/BP_Track.BP_Track_C|GetClosed%20Loop _output_get_2))
        (Variables|Default|SetTrack%20Length (Spline|GetSplineLength _output_get_3))
        (Variables|Default|SetDouble%20Track%20Spacing (Variables|/Game/Railway_System/Blueprints/BP_Track.BP_Track_C|GetDoubleTrack%20Spacing _output_get_2)))
      (:then_1
        ;[1 1 1] Set position on Track
        (bind _distance_on_spline (CallFunction|SearchNearestDistanceonSpline (Variables|Default|GetSpline) (Transformation|GetWorldLocation (Variables|Default|GetDefaultSceneRoot)) 0.5))
        (Variables|Default|SetPosition _distance_on_spline))
      (:then_2
        ;[1 1 1] Set Tunnel length limited by spline position and length
        (if (Variables|Default|GetClosedLoop)
          (Variables|Default|SetResulting%20Length (Math|Float|Clamp(Float) _returnvalue_2 0.0 (Variables|Default|GetTrack%20Length)))
          (else
            (Variables|Default|SetResulting%20Length (Math|Float|Clamp(Float) _returnvalue_2 0.0 (- (Math|Float|SelectFloat (Variables|Default|GetPosition) (- (Variables|Default|GetTrack%20Length) (Variables|Default|GetPosition)) (Variables|Tunnel|GetReverse%20Tunnel%20Direction)) 1.0))))))
      (:then_3
        (for _index (range (Math|Integer|SelectInt (* (Math|Integer|Clamp(Integer) (Math|Float|Truncate (/ (Variables|Default|GetResulting%20Length) (Variables|Default|GetMesh%20Length))) 1 10000) -1) 0 _reverse_tunnel_direction) (Math|Integer|SelectInt -1 (- (Math|Integer|Clamp(Integer) (Math|Float|Truncate (/ (Variables|Default|GetResulting%20Length) (Variables|Default|GetMesh%20Length))) 1 10000) 1) _reverse_tunnel_direction))
          ;[1 1 1] Add and setup spline meshes
          (bind _returnvalue_4 (AddComponent|AddSplineMeshComponent false))
          (if (Variables|Default|GetDoubleTrack)
            (Components|StaticMesh|SetStaticMesh _returnvalue_4 "/Game/Railway_System/Meshes/Tunnel/SM_Tunnel_DoubleTrack.SM_Tunnel_DoubleTrack"))
          (SplineMesh|SetStartandEnd _returnvalue_4 (+ (select (Variables|Default|GetDoubleTrack) (- (Spline|GetLocationatDistanceAlongSpline (Variables|Default|GetSpline) (Utilities|SplineModulo (+ (* _index (/ (Variables|Default|GetResulting%20Length) (Math|Conversions|ToFloat(Integer) (Math|Integer|Clamp(Integer) (Math|Float|Truncate (/ (Variables|Default|GetResulting%20Length) (Variables|Default|GetMesh%20Length))) 1 10000)))) (Variables|Default|GetPosition))) "World") (* (Class|SplineComponent|GetRightVectoratDistanceAlongSpline (Variables|Default|GetSpline) (Utilities|SplineModulo (+ (* _index (/ (Variables|Default|GetResulting%20Length) (Math|Conversions|ToFloat(Integer) (Math|Integer|Clamp(Integer) (Math|Float|Truncate (/ (Variables|Default|GetResulting%20Length) (Variables|Default|GetMesh%20Length))) 1 10000)))) (Variables|Default|GetPosition))) "World") (/ (Variables|Default|GetDouble%20Track%20Spacing) 2.0))) (Spline|GetLocationatDistanceAlongSpline (Variables|Default|GetSpline) (Utilities|SplineModulo (+ (* _index (/ (Variables|Default|GetResulting%20Length) (Math|Conversions|ToFloat(Integer) (Math|Integer|Clamp(Integer) (Math|Float|Truncate (/ (Variables|Default|GetResulting%20Length) (Variables|Default|GetMesh%20Length))) 1 10000)))) (Variables|Default|GetPosition))) "World")) (Math|Vector|MakeVector 0.0 0.0 (Variables|Default|GetRail%20Top%20Height)) _returnvalue_3) (* (Math|Vector|Normalize (Spline|GetTangentatDistanceAlongSpline (Variables|Default|GetSpline) (Utilities|SplineModulo (+ (* _index (/ (Variables|Default|GetResulting%20Length) (Math|Conversions|ToFloat(Integer) (Math|Integer|Clamp(Integer) (Math|Float|Truncate (/ (Variables|Default|GetResulting%20Length) (Variables|Default|GetMesh%20Length))) 1 10000)))) (Variables|Default|GetPosition))) "World")) _mesh_length) (+ (select (Variables|Default|GetDoubleTrack) (- (Spline|GetLocationatDistanceAlongSpline (Variables|Default|GetSpline) (Math|Float|Clamp(Float) (Utilities|SplineModulo (+ (* (+ _index 1) (/ (Variables|Default|GetResulting%20Length) (Math|Conversions|ToFloat(Integer) (Math|Integer|Clamp(Integer) (Math|Float|Truncate (/ (Variables|Default|GetResulting%20Length) (Variables|Default|GetMesh%20Length))) 1 10000)))) (Variables|Default|GetPosition))) 0.0 (- (Variables|Default|GetTrack%20Length) 1.0)) "World") (* (Class|SplineComponent|GetRightVectoratDistanceAlongSpline (Variables|Default|GetSpline) (Math|Float|Clamp(Float) (Utilities|SplineModulo (+ (* (+ _index 1) (/ (Variables|Default|GetResulting%20Length) (Math|Conversions|ToFloat(Integer) (Math|Integer|Clamp(Integer) (Math|Float|Truncate (/ (Variables|Default|GetResulting%20Length) (Variables|Default|GetMesh%20Length))) 1 10000)))) (Variables|Default|GetPosition))) 0.0 (- (Variables|Default|GetTrack%20Length) 1.0)) "World") (/ (Variables|Default|GetDouble%20Track%20Spacing) 2.0))) (Spline|GetLocationatDistanceAlongSpline (Variables|Default|GetSpline) (Math|Float|Clamp(Float) (Utilities|SplineModulo (+ (* (+ _index 1) (/ (Variables|Default|GetResulting%20Length) (Math|Conversions|ToFloat(Integer) (Math|Integer|Clamp(Integer) (Math|Float|Truncate (/ (Variables|Default|GetResulting%20Length) (Variables|Default|GetMesh%20Length))) 1 10000)))) (Variables|Default|GetPosition))) 0.0 (- (Variables|Default|GetTrack%20Length) 1.0)) "World")) (Math|Vector|MakeVector 0.0 0.0 (Variables|Default|GetRail%20Top%20Height)) _returnvalue_3) (* (Math|Vector|Normalize (Spline|GetTangentatDistanceAlongSpline (Variables|Default|GetSpline) (Math|Float|Clamp(Float) (Utilities|SplineModulo (+ (* (+ _index 1) (/ (Variables|Default|GetResulting%20Length) (Math|Conversions|ToFloat(Integer) (Math|Integer|Clamp(Integer) (Math|Float|Truncate (/ (Variables|Default|GetResulting%20Length) (Variables|Default|GetMesh%20Length))) 1 10000)))) (Variables|Default|GetPosition))) 0.0 (- (Variables|Default|GetTrack%20Length) 1.0)) "World")) _mesh_length) true :!class /Script/Engine.SplineMeshComponent)
          (Rendering|Material|SetScalarParameterValueonMaterials _returnvalue_4 "Emissive" (Variables|Tunnel|GetLights%20Emissive))))
      (:then_4
        ;[1 1 1] Add Portals
        (CallFunction|AddPortal (select _reverse_tunnel_direction_2 (- (Variables|Default|GetPosition) (Variables|Default|GetResulting%20Length)) (Variables|Default|GetPosition)) false)
        (CallFunction|AddPortal (select _reverse_tunnel_direction_2 (Variables|Default|GetPosition) (+ (Variables|Default|GetPosition) (Variables|Default|GetResulting%20Length))) true)))
    (else
      (AddComponent|AddTextRenderComponent false))))

(fn AddPortal
  (params (Position :type Float%20%28single-precision%29) (End :type Boolean))
  (bind _position_in_spline_range (Utilities|SplineModulo Position))
  (bind _self self)
  (bind _rail_top_height (Variables|Default|GetRail%20Top%20Height))
  (bind _double_track_spacing (Variables|Default|GetDouble%20Track%20Spacing))
  (bind _spline (Variables|Default|GetSpline))
  (bind _doubletrack (Variables|Default|GetDoubleTrack))
  (bind _returnvalue (Math|Vector|MakeVector 0.0 0.0 _rail_top_height))
  (bind _returnvalue_2 (Spline|GetDirectionatDistanceAlongSpline _spline _position_in_spline_range "World"))
  (bind _returnvalue_3 (Spline|GetLocationatDistanceAlongSpline _spline _position_in_spline_range "World"))
  (bind _returnvalue_4 (Class|SplineComponent|GetRightVectoratDistanceAlongSpline _spline _position_in_spline_range "World"))
  (bind _returnvalue_5 (/ _double_track_spacing 2.0))
  (bind _defaultsceneroot (Variables|Default|GetDefaultSceneRoot _self))
  (bind _returnvalue_6 (Transformation|GetWorldLocation _defaultsceneroot))
  (bind _returnvalue_7 (Transformation|GetWorldRotation _defaultsceneroot))
  (bind _returnvalue_8 (* _returnvalue_2 -1.0))
  (bind _returnvalue_9 (* _returnvalue_4 _returnvalue_5))
  (bind _returnvalue_10 (Math|Conversions|RotationFromXVector _returnvalue_8))
  (bind _returnvalue_11 (- _returnvalue_3 _returnvalue_9))
  (bind _returnvalue_12 (Math|Rotator|Delta(Rotator) _returnvalue_10 _returnvalue_7))
  (bind _returnvalue_13 (Math|Vector|SelectVector _returnvalue_11 _returnvalue_3 _doubletrack))
  (bind _returnvalue_14 (- _returnvalue_13 _returnvalue_6))
  (bind _returnvalue_15 (+ _returnvalue _returnvalue_14))
  (bind _returnvalue_16 (AddComponent|AddStaticMeshComponent false (Math|Transform|MakeTransform _returnvalue_15 _returnvalue_12 (Math|Vector|MakeVector (Variables|Tunnel|GetPortals%20Long%20Scaling) 1.0 1.0))))
  (if (Variables|Default|GetDoubleTrack)
    (Components|StaticMesh|SetStaticMesh _returnvalue_16 "/Game/Railway_System/Meshes/Tunnel/SM_Tunnel_Portal_DoubleTrack.SM_Tunnel_Portal_DoubleTrack"))
  (if End
    (Transformation|AddLocalRotation _returnvalue_16 "0.000000,180.000000,0.000000" false false))
  ;[1 1 1] Block Entrance
  (if (Variables|Tunnel|GetBlock%20Entrance)
    (bind _returnvalue_17 (AddComponent|AddBoxComponent false (Math|Transform|MakeTransform _returnvalue_15 _returnvalue_12 "1,1,1")))
    (Transformation|AddLocalOffset _returnvalue_17 (Math|Vector|MakeVector (* (Variables|Tunnel|GetBlocking%20box%20offset%20inwards%20%28m%29) 1e+02 (Math|Float|SelectFloat 1.0 -1.0 End)) 0.0 0.0) false false)))