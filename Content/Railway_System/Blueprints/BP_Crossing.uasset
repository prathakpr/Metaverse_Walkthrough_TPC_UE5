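; BP_Crossing is a railway level crossing that snaps onto the nearest BP_Track spline, placing crossing meshes and signals for single or double track.
; In automatic mode, Tick estimates each same-track train's time to the crossing on a wrapping track, using shrinking distance to detect approach.
; Closing starts sounds and emissive lights, then optionally lowers physics-constraint gates by timeline after a delay.
; Opening stops sounds and reverses the gates, turning lights off once they finish.
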(event Custom|Open%20Crossing
  ;[1 1 1] Open and Close Events
  (Default|CallCrossingStartstoOpen)
  (Variables|CrossingConfiguration|SetIs%20Closed false)
  (Audio|Components|Audio|Stop (Variables|Default|GetSound_Crossing1))
  (if (Variables|CrossingConfiguration|GetCrossing%20Gates)
    (Class|PrimitiveComponent|WakeRigidBody (Variables|Default|GetCrossing_Gate1) "None")
    (bind _newtrack_0 (Timeline|CrossingGate Reverse)
      (:Update
        (Class|PhysicsConstraintComponent|SetAngularOrientationTarget (Variables|Default|GetPhysicsConstraint1) (Math|Rotator|MakeRotator 0.0 (+ (* _newtrack_0 -86.0) 43.0) 0.0)))
      (:Finished
        (if (not (Variables|CrossingConfiguration|GetIs%20Closed))
          (Rendering|Material|SetScalarParameterValueonMaterials (Variables|Default|GetCrossing_Signal1) "Emissive" 0.0 :!label _label))))
    (else
      (goto _label))))

(event Custom|Close%20Crossing
  ;[1 1 1] Open and Close Events
  (Default|CallCrossingStartstoClose)
  (Variables|CrossingConfiguration|SetIs%20Closed true)
  (Audio|Components|Audio|Play (Variables|Default|GetSound_Crossing1) 0.0)
  (Rendering|Material|SetScalarParameterValueonMaterials (Variables|Default|GetCrossing_Signal1) "Emissive" 5.0)
  (if (Variables|CrossingConfiguration|GetCrossing%20Gates)
    (Utilities|FlowControl|Delay (Variables|CrossingConfiguration|GetDelay%20before%20closing%20Gate))
    (if (Variables|CrossingConfiguration|GetIs%20Closed)
      (Class|PrimitiveComponent|WakeRigidBody (Variables|Default|GetCrossing_Gate1) "None")
      (bind _newtrack_0 (Timeline|CrossingGate Play)
        (:Update
          (Class|PhysicsConstraintComponent|SetAngularOrientationTarget (Variables|Default|GetPhysicsConstraint1) (Math|Rotator|MakeRotator 0.0 (+ (* _newtrack_0 -86.0) 43.0) 0.0)))
        (:Finished
          (if (not (Variables|CrossingConfiguration|GetIs%20Closed))
            (Rendering|Material|SetScalarParameterValueonMaterials (Variables|Default|GetCrossing_Signal1) "Emissive" 0.0)))))))

(event EventBeginPlay
  (CallFunction|GetAllTrainsonTrack)
  (if (and (Variables|CrossingConfiguration|GetIs%20Closed) (not (Variables|AutomaticMode|GetAutomatic%20Mode)))
    (CallFunction|CloseCrossing)))

(event EventTick
  (params (DeltaSeconds :type Float%20%28single-precision%29))
  (if (Variables|AutomaticMode|GetAutomatic%20Mode)
    (Utilities|FlowControl|Sequence
      (:then_0
        ;[1 1 1] Time before/after closest Train
        (Variables|AutomaticMode|SetMin%20Time 2e+02)
        (Variables|AutomaticMode|SetMin%20Distance (Variables|Default|GetTrack%20Length))
        (for _array_element (Variables|Default|GetTrains)
          (if (< (/ (- (Math|Float|Min(Float) (- (Variables|Default|GetTrack%20Length) (Math|Float|Absolute(Float) (- (Utilities|Modulo (Variables|Default|GetPosition)) (Utilities|Modulo (Math|Float|SelectFloat (- (Variables|Default|GetTrack%20Length) (Variables|/Game/Railway_System/Blueprints/BP_Train.BP_Train_C|GetPosition _array_element)) (Variables|/Game/Railway_System/Blueprints/BP_Train.BP_Train_C|GetPosition _array_element) (Variables|/Game/Railway_System/Blueprints/BP_Train.BP_Train_C|GetIs%20on%20Second%20Track _array_element)))))) (Math|Float|Absolute(Float) (- (Utilities|Modulo (Variables|Default|GetPosition)) (Utilities|Modulo (Math|Float|SelectFloat (- (Variables|Default|GetTrack%20Length) (Variables|/Game/Railway_System/Blueprints/BP_Train.BP_Train_C|GetPosition _array_element)) (Variables|/Game/Railway_System/Blueprints/BP_Train.BP_Train_C|GetPosition _array_element) (Variables|/Game/Railway_System/Blueprints/BP_Train.BP_Train_C|GetIs%20on%20Second%20Track _array_element)))))) (Variables|/Game/Railway_System/Blueprints/BP_Train.BP_Train_C|GetHalf%20Train%20Length _array_element)) (+ (Variables|/Game/Railway_System/Blueprints/BP_Train.BP_Train_C|GetCurrent%20Speed _array_element) 1.0)) (Variables|AutomaticMode|GetMin%20Time))
            (Variables|AutomaticMode|SetMin%20Time (/ (- (Math|Float|Min(Float) (- (Variables|Default|GetTrack%20Length) (Math|Float|Absolute(Float) (- (Utilities|Modulo (Variables|Default|GetPosition)) (Utilities|Modulo (Math|Float|SelectFloat (- (Variables|Default|GetTrack%20Length) (Variables|/Game/Railway_System/Blueprints/BP_Train.BP_Train_C|GetPosition _array_element)) (Variables|/Game/Railway_System/Blueprints/BP_Train.BP_Train_C|GetPosition _array_element) (Variables|/Game/Railway_System/Blueprints/BP_Train.BP_Train_C|GetIs%20on%20Second%20Track _array_element)))))) (Math|Float|Absolute(Float) (- (Utilities|Modulo (Variables|Default|GetPosition)) (Utilities|Modulo (Math|Float|SelectFloat (- (Variables|Default|GetTrack%20Length) (Variables|/Game/Railway_System/Blueprints/BP_Train.BP_Train_C|GetPosition _array_element)) (Variables|/Game/Railway_System/Blueprints/BP_Train.BP_Train_C|GetPosition _array_element) (Variables|/Game/Railway_System/Blueprints/BP_Train.BP_Train_C|GetIs%20on%20Second%20Track _array_element)))))) (Variables|/Game/Railway_System/Blueprints/BP_Train.BP_Train_C|GetHalf%20Train%20Length _array_element)) (+ (Variables|/Game/Railway_System/Blueprints/BP_Train.BP_Train_C|GetCurrent%20Speed _array_element) 1.0)))
            (Variables|AutomaticMode|SetMin%20Distance (Math|Float|Min(Float) (- (Variables|Default|GetTrack%20Length) (Math|Float|Absolute(Float) (- (Utilities|Modulo (Variables|Default|GetPosition)) (Utilities|Modulo (Math|Float|SelectFloat (- (Variables|Default|GetTrack%20Length) (Variables|/Game/Railway_System/Blueprints/BP_Train.BP_Train_C|GetPosition _array_element)) (Variables|/Game/Railway_System/Blueprints/BP_Train.BP_Train_C|GetPosition _array_element) (Variables|/Game/Railway_System/Blueprints/BP_Train.BP_Train_C|GetIs%20on%20Second%20Track _array_element)))))) (Math|Float|Absolute(Float) (- (Utilities|Modulo (Variables|Default|GetPosition)) (Utilities|Modulo (Math|Float|SelectFloat (- (Variables|Default|GetTrack%20Length) (Variables|/Game/Railway_System/Blueprints/BP_Train.BP_Train_C|GetPosition _array_element)) (Variables|/Game/Railway_System/Blueprints/BP_Train.BP_Train_C|GetPosition _array_element) (Variables|/Game/Railway_System/Blueprints/BP_Train.BP_Train_C|GetIs%20on%20Second%20Track _array_element))))))))))
      (:then_1
        ;[1 1 1] is Train approaching or leaving?
        (Variables|AutomaticMode|SetTrain%20is%20approaching (< (Variables|AutomaticMode|GetMin%20Distance) (Variables|AutomaticMode|GetLast%20Min%20Distance)))
        (Variables|AutomaticMode|SetLast%20Min%20Distance (Variables|AutomaticMode|GetMin%20Distance)))
      (:then_2
        ;[1 1 1] should Crossing be closed now?
        (Variables|AutomaticMode|SetMust%20be%20Closed (or (and (< (Variables|AutomaticMode|GetMin%20Time) (Variables|AutomaticMode|GetTime%20before%20Train%20for%20closure)) (Variables|AutomaticMode|GetTrain%20is%20approaching)) (and (not (Variables|AutomaticMode|GetTrain%20is%20approaching)) (< (Variables|AutomaticMode|GetMin%20Time) (Variables|AutomaticMode|GetTime%20after%20Train%20for%20opening))))))
      (:then_3
        ;[1 1 1] Open or Close Crossing
        (Utilities|FlowControl|Sequence
          (:then_0
            (if (and (Variables|AutomaticMode|GetMust%20be%20Closed) (not (Variables|CrossingConfiguration|GetIs%20Closed)))
              (CallFunction|CloseCrossing)))
          (:then_1
            (if (and (not (Variables|AutomaticMode|GetMust%20be%20Closed)) (Variables|CrossingConfiguration|GetIs%20Closed))
              (CallFunction|OpenCrossing))))))))

(fn ConstructionScript
  (Variables|CrossingConfiguration|SetUpdate false)
  ;[1 1 1] Search for BP_Track and create message if search failed
  (bind (_track_selected _track_pick) (CallFunction|SearchNearestBPTrack (Transformation|GetWorldLocation (Variables|Default|GetDefaultSceneRoot))))
  (bind _output_get (Variables|Default|SetTrackSelected _track_selected))
  (if _output_get
    (Variables|Default|SetTrack%20Pick _track_pick)
    (Utilities|FlowControl|Sequence
      (:then_0
        ;[1 1 1] Get needed variables from BP_Track
        (Variables|Default|SetSpline (Variables|/Game/Railway_System/Blueprints/BP_Track.BP_Track_C|GetSpline_Current (Variables|Default|GetTrack%20Pick)))
        (Variables|Default|SetRail%20Top%20Height (Variables|/Game/Railway_System/Blueprints/BP_Track.BP_Track_C|GetRail%20Top%20Height (Variables|Default|GetTrack%20Pick)))
        (Variables|Default|SetDoubleTrack (Variables|/Game/Railway_System/Blueprints/BP_Track.BP_Track_C|GetDouble%20Track (Variables|Default|GetTrack%20Pick)))
        (Variables|Default|SetDouble%20Track%20Spacing (Variables|/Game/Railway_System/Blueprints/BP_Track.BP_Track_C|GetDoubleTrack%20Spacing (Variables|Default|GetTrack%20Pick)))
        (Variables|Default|SetTrack%20Length (* (Variables|/Game/Railway_System/Blueprints/BP_Track.BP_Track_C|GetTrack%20Length%20%28m%29 (Variables|Default|GetTrack%20Pick)) 1e+02)))
      (:then_1
        ;[1 1 1] Set position on Track
        (bind _distance_on_spline (CallFunction|SearchNearestDistanceonSpline (Variables|Default|GetSpline) (Transformation|GetWorldLocation (Variables|Default|GetDefaultSceneRoot)) 0.3))
        (Variables|Default|SetPosition _distance_on_spline))
      (:then_2
        ;[1 1 1] Add crossing mesh
        (if (Variables|Default|GetDoubleTrack)
          (CallFunction|AddCrossingMesh false)
          (CallFunction|AddCrossingMesh true)
          (else
            (CallFunction|AddCrossingMesh false))))
      (:then_3
        (Utilities|FlowControl|Sequence
          (:then_0
            (CallFunction|PositionSignal)
            ;[1 1 1] Gate Setup
            (if (Variables|CrossingConfiguration|GetCrossing%20Gates)
              (Transformation|SetRelativeScale3D (Variables|Default|GetCrossing_Gate1) (Math|Vector|MakeVector (/ (Variables|CrossingConfiguration|GetGate%20Length) 4.42) 1.0 1.0))
              (else
                (Components|DestroyComponent (Variables|Default|GetCrossing_Gate1)))))
          (:then_1
            ;[1 1 1] Lights on/off
            (Rendering|Material|SetScalarParameterValueonMaterials (Variables|Default|GetCrossing_Signal1) "Emissive" (* (Math|Conversions|ToFloat(Boolean) (Variables|CrossingConfiguration|GetIs%20Closed)) 5.0)))
          (:then_2
            ;[1 1 1] Audio Volume
            (Audio|Components|Audio|SetVolumeMultiplier (Variables|Default|GetSound_Crossing2) (Variables|CrossingConfiguration|GetSound%20Volume) :!class /Script/Engine.AudioComponent)))))
    (else
      (AddComponent|AddTextRenderComponent false))))

(fn AddCrossingMesh
  (params (SecondTrack :type Boolean))
  (bind _returnvalue (AddComponent|AddStaticMeshComponent false (Utilities|CrossingMeshTransform SecondTrack)))
  (Utilities|Array|Add (Variables|Default|GetCrossing%20Meshes%20Array) _returnvalue)
  (return))

(fn PositionSignal
  (bind (_location _location__second_track_ _rotator) (Utilities|TransformfromPositiononSpline))
  (bind _crossing_signal1 (Variables|Default|GetCrossing_Signal1))
  (bind (_roll _pitch _yaw) (Math|Rotator|BreakRotator _rotator))
  (bind _returnvalue (Math|Rotator|MakeRotator _roll 0.0 _yaw))
  (Transformation|SetWorldTransform _crossing_signal1 (Math|Transform|MakeTransform _location _returnvalue "1,1,1") false true)
  (Transformation|SetWorldTransform (Variables|Default|GetCrossing_Signal2) (Math|Transform|MakeTransform (select (Variables|Default|GetDoubleTrack) _location__second_track_ _location) (Math|Rotator|CombineRotators _returnvalue "0,180.000000, 0") "1,1,1") false true)
  (Transformation|AddLocalOffset _crossing_signal1 (Variables|CrossingConfiguration|GetGate%20Position) false true))

(fn GetAllTrainsonTrack
  (if (Variables|AutomaticMode|GetAutomatic%20Mode)
    (Utilities|Array|Clear (Variables|Default|GetTrains))
    (bind _outactors (Actor|GetAllActorsOfClass "/Game/Railway_System/Blueprints/BP_Train.BP_Train_C"))
    (for _array_element _outactors
      (if (== (Variables|Default|GetTrack%20Pick) (Variables|/Game/Railway_System/Blueprints/BP_Train.BP_Train_C|GetTrack%20Pick _array_element))
        (Utilities|Array|Add (Variables|Default|GetTrains) _array_element)))))