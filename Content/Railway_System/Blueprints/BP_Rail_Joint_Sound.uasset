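; BP_Rail_Joint_Sound is a railway actor that plays a rail joint sound as train wheels pass over it.
; Its Sphere's begin overlap filters for components with "Wheel" in their display name and casts their owner to BP_Train.
; The train's CurrentSpeed drives the attenuated one-shot at the sphere's location: clamped volume follows squared normalized speed, scaled by VolumeMultiplier, while clamped pitch rises linearly.
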(event OnComponentBeginOverlap(Sphere)
  (params (OverlappedComponent :type Primitive%20Component%20Object%20Reference) (OtherActor :type Actor%20Object%20Reference) (OtherComp :type Primitive%20Component%20Object%20Reference) (OtherBodyIndex :type Integer) (bFromSweep :type Boolean) (SweepResult :type Hit%20Result%20Structure%20%28by%20ref%29))
  (if (>= (Utilities|String|FindSubstring (Utilities|GetDisplayName OtherComp) "Wheel" false true) 0)
    (bind _asbp_train (Utilities|Casting|CastToBP_Train (Components|GetOwner OtherComp)))
    (Audio|PlaySoundatLocation "/Game/Railway_System/Sound/SC_RailJoint.SC_RailJoint" (Transformation|GetWorldLocation (Variables|Default|GetSphere)) "0, 0, 0" (* (Math|Float|Clamp(Float) (Math|Float|Lerp -0.2 1.0 (Math|Float|Square (/ (Variables|/Game/Railway_System/Blueprints/BP_Train.BP_Train_C|GetCurrent%20Speed _asbp_train) 2222.0)))) (Variables|RailJoint|GetVolume%20Multiplier)) (Math|Float|Clamp(Float) (Math|Float|Lerp 0.2 1.0 (/ (Variables|/Game/Railway_System/Blueprints/BP_Train.BP_Train_C|GetCurrent%20Speed _asbp_train) 2222.0)) 0.2 1.1) 0.0 "/Game/Railway_System/Sound/TrainSoundAttenuation.TrainSoundAttenuation" 0 0)))

(event EventBeginPlay)

(event Collision|EventActorBeginOverlap
  (params (OtherActor :type Actor%20Object%20Reference)))

(event EventTick
  (params (DeltaSeconds :type Float%20%28single-precision%29)))

(fn ConstructionScript)