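; BP_Switch is a railway switch actor that moves trains onto another track when they touch its trigger sphere.
; On sphere overlap, while active and with a valid target track, it casts the actor to BP_Train.
; If the train is not already on that track, it fires a TrainChangedTrack event and calls ChangeTrack, passing the second-track and reverse-direction settings.
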(event OnComponentBeginOverlap(Sphere)
  (params (OverlappedComponent :type Primitive%20Component%20Object%20Reference) (OtherActor :type Actor%20Object%20Reference) (OtherComp :type Primitive%20Component%20Object%20Reference) (OtherBodyIndex :type Integer) (bFromSweep :type Boolean) (SweepResult :type Hit%20Result%20Structure%20%28by%20ref%29))
  (if (and (Variables|Switch|GetActive) (Utilities|IsValid (Variables|Switch|GetTrack%20to%20change%20to)))
    (bind _asbp_train (Utilities|Casting|CastToBP_Train OtherActor))
    ;[1 1 1] Whether new Track is not equal to old Track
    (if (not (== (Variables|/Game/Railway_System/Blueprints/BP_Train.BP_Train_C|GetTrack%20Pick _asbp_train) (Variables|Switch|GetTrack%20to%20change%20to)))
      (Default|CallTrainChangedTrack _asbp_train)
      ;[1 1 1] Change Train's Track
      (Default|ChangeTrack _asbp_train (Variables|Switch|GetTrack%20to%20change%20to) (Variables|Switch|GetChange%20to%20Second%20Track) (Variables|Switch|GetReverse%20Direction)))))

(event EventBeginPlay)

(event Collision|EventActorBeginOverlap
  (params (OtherActor :type Actor%20Object%20Reference)))

(event EventTick
  (params (DeltaSeconds :type Float%20%28single-precision%29)))

(fn ConstructionScript)