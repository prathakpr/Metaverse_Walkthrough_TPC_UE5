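; Railway station platform actor that snaps to the nearest BP_Track and builds itself along that track's spline in the construction script, with no runtime logic.
; It clamps length and position to the track, then lays spline mesh segments on one side, or both for double track, with end steps and optional pedestrian crossings.
; Segment sockets carry optional instanced fences, shelters with seating, bins and spotlights, and name signs at set spacing.
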(event EventBeginPlay)

(event Collision|EventActorBeginOverlap
  (params (OtherActor :type Actor%20Object%20Reference)))

(event EventTick
  (params (DeltaSeconds :type Float%20%28single-precision%29)))

(fn ConstructionScript
  (Variables|Platform|SetUpdate false)
  (Transformation|SetActorRotation "0, 0, 0")
  ;[1 1 1] Search for BP_Track and create message if search failed
  (bind (_track_selected _track_pick) (CallFunction|SearchNearestBPTrack (Transformation|GetWorldLocation (Variables|Default|GetDefaultSceneRoot))))
  (bind _output_get (Variables|Default|SetTrackSelected _track_selected))
  (if _output_get
    (Utilities|FlowControl|Sequence
      (:then_0
        ;[1 1 1] Get needed variables from BP_Track
        (bind _output_get_2 (Variables|Default|SetTrack%20Pick _track_pick))
        (bind _output_get_3 (Variables|Default|SetSpline (Variables|/Game/Railway_System/Blueprints/BP_Track.BP_Track_C|GetSpline_Current _output_get_2)))
        (Variables|Default|SetRail%20Top%20Height (Variables|/Game/Railway_System/Blueprints/BP_Track.BP_Track_C|GetRail%20Top%20Height _output_get_2))
        (Variables|Default|SetDoubleTrack (Variables|/Game/Railway_System/Blueprints/BP_Track.BP_Track_C|GetDouble%20Track _output_get_2))
        (Variables|Default|SetClosedLoop (Variables|/Game/Railway_System/Blueprints/BP_Track.BP_Track_C|GetClosed%20Loop _output_get_2))
        (Variables|Default|SetTrack%20Length (Spline|GetSplineLength _output_get_3))
        (Variables|Default|SetDouble%20Track%20Spacing (Variables|/Game/Railway_System/Blueprints/BP_Track.BP_Track_C|GetDoubleTrack%20Spacing _output_get_2)))
      (:then_1
        ;[1 1 1] Set Platform length limited by spline position and length
        (Variables|Default|SetResulting%20Length (Math|Float|Clamp(Float) (* (Variables|Platform|GetLenght%20%28m%29) 1e+02) 0.0 (- (Variables|Default|GetTrack%20Length) 5e+02))))
      (:then_2
        ;[1 1 1] Set position on Track
        (bind _distance_on_spline (CallFunction|SearchNearestDistanceonSpline (Variables|Default|GetSpline) (Transformation|GetWorldLocation (Variables|Default|GetDefaultSceneRoot)) 0.5))
        (Variables|Default|SetPosition (select (Variables|Default|GetClosedLoop) _distance_on_spline (Math|Float|Clamp(Float) _distance_on_spline (/ (Variables|Default|GetResulting%20Length) 2.0) (- (- (Variables|Default|GetTrack%20Length) (/ (Variables|Default|GetResulting%20Length) 2.0)) 1e+02))))
        (Variables|Default|SetWorld%20Position (Spline|GetLocationatDistanceAlongSpline (Variables|Default|GetSpline) _distance_on_spline "World")))
      (:then_3
        ;[1 1 1] Platform meshes
        (if (Variables|Default|GetDoubleTrack)
          (Variables|Platform|SetOpposite%20Side true)
          (CallFunction|AddMeshes)
          (Variables|Platform|SetOpposite%20Side false)
          (CallFunction|AddMeshes)
          (else
            (CallFunction|AddMeshes))))
      (:then_4
        ;[1 1 1] Steps
        (if (Variables|Default|GetDoubleTrack)
          (CallFunction|AddSteps false false)
          (CallFunction|AddSteps true false)
          (CallFunction|AddSteps false true)
          (CallFunction|AddSteps true true)
          (else
            (CallFunction|AddSteps (Variables|Platform|GetOpposite%20Side) false)
            (CallFunction|AddSteps (Variables|Platform|GetOpposite%20Side) true)))))
    (else
      (AddComponent|AddTextRenderComponent false))))

(fn AddMeshes
  (bind _opposite_side (Variables|Platform|GetOpposite%20Side))
  (bind _spline (Variables|Default|GetSpline))
  (bind _mesh_length (Variables|Default|GetMesh%20Length))
  (bind _defaultsceneroot (Variables|Default|GetDefaultSceneRoot))
  (bind _position (Variables|Default|GetPosition))
  (bind _opposite_side_2 (Variables|Platform|GetOpposite%20Side))
  (bind _opposite_side_3 (Variables|Platform|GetOpposite%20Side))
  (bind _rail_top_height (Variables|Default|GetRail%20Top%20Height))
  (bind _doubletrack (Variables|Default|GetDoubleTrack))
  (bind _double_track_spacing (Variables|Default|GetDouble%20Track%20Spacing))
  (bind _adjust_lateral_position (Variables|Platform|GetAdjust%20Lateral%20Position))
  (bind _shelter_spacing (Variables|AdditionalMeshes|GetShelter%20Spacing))
  (bind _sign_spacing (Variables|Name|GetSign%20Spacing))
  (bind _opposite_side_4 (Variables|Platform|GetOpposite%20Side))
  (bind _resulting_length (Variables|Default|GetResulting%20Length))
  (bind _returnvalue (/ _resulting_length 2.0))
  (bind _returnvalue_2 (Math|Vector|MakeVector 0.0 0.0 _rail_top_height))
  (bind _returnvalue_3 (Transformation|GetWorldLocation _defaultsceneroot))
  (bind _returnvalue_4 (and _doubletrack _opposite_side_3))
  (bind _returnvalue_5 (select _opposite_side -1.0 1.0))
  (bind _returnvalue_6 (select _opposite_side_4 1.0 -1.0))
  (bind _returnvalue_7 (- _position _returnvalue))
  (bind _returnvalue_8 (Math|Conversions|ToFloat(Boolean) _returnvalue_4))
  (bind _returnvalue_9 (* _returnvalue_3 -1.0))
  (bind _returnvalue_10 (* _mesh_length _returnvalue_5))
  (bind _returnvalue_11 (* _adjust_lateral_position _returnvalue_6))
  (bind _returnvalue_12 (* _double_track_spacing _returnvalue_8))
  (bind _returnvalue_13 (+ _returnvalue_12 _returnvalue_11))
  ;[1 1 1] Number of Meshes
  (Variables|Default|SetNum%20p%20m (Math|Integer|Clamp(Integer) (Math|Float|Truncate (/ (Variables|Default|GetResulting%20Length) (Variables|Default|GetMesh%20Length))) 1 10000))
  (for _index (range 0 (- (Variables|Default|GetNum%20p%20m) 1))
    ;[1 1 1] Add Platform base meshes
    (bind _returnvalue_14 (AddComponent|AddSplineMeshComponent false))
    (Utilities|Array|Add (Variables|Default|GetPlatform%20Base%20Meshes) _returnvalue_14)
    (SplineMesh|SetStartandEnd _returnvalue_14 (+ (- (Spline|GetLocationatDistanceAlongSpline _spline (select _opposite_side_2 (Math|Float|Clamp(Float) (Utilities|SplineModulo (+ (* (+ _index 1) (/ (Variables|Default|GetResulting%20Length) (Math|Conversions|ToFloat(Integer) (Variables|Default|GetNum%20p%20m)))) _returnvalue_7)) 0.0 (- (Variables|Default|GetTrack%20Length) 1.0)) (Utilities|SplineModulo (+ (* _index (/ (Variables|Default|GetResulting%20Length) (Math|Conversions|ToFloat(Integer) (Variables|Default|GetNum%20p%20m)))) _returnvalue_7))) "World") (* (Class|SplineComponent|GetRightVectoratDistanceAlongSpline _spline (select _opposite_side_2 (Math|Float|Clamp(Float) (Utilities|SplineModulo (+ (* (+ _index 1) (/ (Variables|Default|GetResulting%20Length) (Math|Conversions|ToFloat(Integer) (Variables|Default|GetNum%20p%20m)))) _returnvalue_7)) 0.0 (- (Variables|Default|GetTrack%20Length) 1.0)) (Utilities|SplineModulo (+ (* _index (/ (Variables|Default|GetResulting%20Length) (Math|Conversions|ToFloat(Integer) (Variables|Default|GetNum%20p%20m)))) _returnvalue_7))) "World") _returnvalue_13)) _returnvalue_2 _returnvalue_9) (* (Math|Vector|Normalize (Spline|GetTangentatDistanceAlongSpline _spline (select _opposite_side_2 (Math|Float|Clamp(Float) (Utilities|SplineModulo (+ (* (+ _index 1) (/ (Variables|Default|GetResulting%20Length) (Math|Conversions|ToFloat(Integer) (Variables|Default|GetNum%20p%20m)))) _returnvalue_7)) 0.0 (- (Variables|Default|GetTrack%20Length) 1.0)) (Utilities|SplineModulo (+ (* _index (/ (Variables|Default|GetResulting%20Length) (Math|Conversions|ToFloat(Integer) (Variables|Default|GetNum%20p%20m)))) _returnvalue_7))) "World")) _returnvalue_10) (+ (- (Spline|GetLocationatDistanceAlongSpline _spline (select _opposite_side_2 (Utilities|SplineModulo (+ (* _index (/ (Variables|Default|GetResulting%20Length) (Math|Conversions|ToFloat(Integer) (Variables|Default|GetNum%20p%20m)))) _returnvalue_7)) (Math|Float|Clamp(Float) (Utilities|SplineModulo (+ (* (+ _index 1) (/ (Variables|Default|GetResulting%20Length) (Math|Conversions|ToFloat(Integer) (Variables|Default|GetNum%20p%20m)))) _returnvalue_7)) 0.0 (- (Variables|Default|GetTrack%20Length) 1.0))) "World") (* (Class|SplineComponent|GetRightVectoratDistanceAlongSpline _spline (select _opposite_side_2 (Utilities|SplineModulo (+ (* _index (/ (Variables|Default|GetResulting%20Length) (Math|Conversions|ToFloat(Integer) (Variables|Default|GetNum%20p%20m)))) _returnvalue_7)) (Math|Float|Clamp(Float) (Utilities|SplineModulo (+ (* (+ _index 1) (/ (Variables|Default|GetResulting%20Length) (Math|Conversions|ToFloat(Integer) (Variables|Default|GetNum%20p%20m)))) _returnvalue_7)) 0.0 (- (Variables|Default|GetTrack%20Length) 1.0))) "World") _returnvalue_13)) _returnvalue_2 _returnvalue_9) (* (Math|Vector|Normalize (Spline|GetTangentatDistanceAlongSpline _spline (select _opposite_side_2 (Utilities|SplineModulo (+ (* _index (/ (Variables|Default|GetResulting%20Length) (Math|Conversions|ToFloat(Integer) (Variables|Default|GetNum%20p%20m)))) _returnvalue_7)) (Math|Float|Clamp(Float) (Utilities|SplineModulo (+ (* (+ _index 1) (/ (Variables|Default|GetResulting%20Length) (Math|Conversions|ToFloat(Integer) (Variables|Default|GetNum%20p%20m)))) _returnvalue_7)) 0.0 (- (Variables|Default|GetTrack%20Length) 1.0))) "World")) _returnvalue_10) true :!class /Script/Engine.SplineMeshComponent)
    (Rendering|Material|SetVectorParameterValueonMaterials _returnvalue_14 "TilesColor" (Math|Conversions|ToVector(LinearColor) (Math|Conversions|ToLinearColor(Color) (Variables|Platform|GetTiles%20Color))))
    (Rendering|Material|SetScalarParameterValueonMaterials _returnvalue_14 "Grunge Contrast" (Variables|Platform|GetTiles%20Grunge%20Contrast))
    (Utilities|FlowControl|Sequence
      (:then_0
        ;[1 1 1] Fence
        (if (Variables|AdditionalMeshes|GetFence)
          (bind _returnvalue_15 (AddComponent|AddInstancedStaticMeshComponent false))
          (bind _output_get (Variables|Default|SetFence%20Instanced%20Mesh _returnvalue_15))
          (CallFunction|AddFences _returnvalue_14)
          (Rendering|Material|SetVectorParameterValueonMaterials _output_get "MetalColor" (Math|Conversions|ToVector(LinearColor) (Math|Conversions|ToLinearColor(Color) (Variables|AdditionalMeshes|GetFence%20Color))))
          (Rendering|Material|SetScalarParameterValueonMaterials _output_get "Additional Roughness" (Variables|AdditionalMeshes|GetFence%20Roughness))))
      (:then_1
        (if (and (== (Math|Integer|%(Integer) (- _index (/ _shelter_spacing 2)) _shelter_spacing) 0) (Variables|AdditionalMeshes|GetShelter))
          ;[1 1 1] Shelter, Seating, Garbage Can
          (bind _returnvalue_16 (AddComponent|AddStaticMeshComponent false))
          (Transformation|AttachComponentToComponent _returnvalue_16 _returnvalue_14 "Shelter" "KeepRelative" "KeepRelative" "KeepRelative" true)
          (Rendering|Material|SetVectorParameterValueonMaterials _returnvalue_16 "MetalColor" (Math|Conversions|ToVector(LinearColor) (Math|Conversions|ToLinearColor(Color) (Variables|AdditionalMeshes|GetShelter%20Color))))
          (Rendering|Material|SetScalarParameterValueonMaterials _returnvalue_16 "Additional Roughness" (Variables|AdditionalMeshes|GetShelter%20Roughness))
          (if (Variables|AdditionalMeshes|GetSeating)
            (bind _returnvalue_17 (AddComponent|AddStaticMeshComponent false))
            (Transformation|AttachComponentToComponent _returnvalue_17 _returnvalue_16 "Seating" "KeepRelative" "KeepRelative" "KeepRelative" true))
          (if (Variables|AdditionalMeshes|GetGarbage_Can)
            (bind _returnvalue_18 (AddComponent|AddStaticMeshComponent false))
            (Transformation|AttachComponentToComponent _returnvalue_18 _returnvalue_16 "Garbage" "KeepRelative" "KeepRelative" "KeepRelative" false))
          ;[1 1 1] Lights
          (if (Variables|AdditionalMeshes|GetShelter%20Lights)
            (bind _returnvalue_19 (AddComponent|AddSpotLightComponent false))
            (Transformation|AttachComponentToComponent _returnvalue_19 _returnvalue_16 "Lamp" "KeepRelative" "KeepRelative" "KeepRelative" true)
            (Rendering|Components|Light|SetIntensity _returnvalue_19 (Variables|AdditionalMeshes|GetLights%20Intensity)))))
      (:then_2
        (if (and (== (Math|Integer|%(Integer) (- _index (/ _sign_spacing 2)) _sign_spacing) 0) (Variables|Name|GetShow%20Platform%20Name%20Sign))
          ;[1 1 1] Platform Name Sign
          (bind _returnvalue_20 (AddComponent|AddStaticMeshComponent false))
          (Transformation|AttachComponentToComponent _returnvalue_20 _returnvalue_14 "Sign" "KeepRelative" "KeepRelative" "KeepRelative" false)
          (Rendering|Material|SetVectorParameterValueonMaterials _returnvalue_20 "MetalColor" (Math|Conversions|ToVector(LinearColor) (Math|Conversions|ToLinearColor(Color) (Variables|AdditionalMeshes|GetShelter%20Color))))
          (Rendering|Material|SetScalarParameterValueonMaterials _returnvalue_20 "Additional Roughness" (Variables|AdditionalMeshes|GetShelter%20Roughness))
          (bind _returnvalue_21 (AddComponent|AddTextRenderComponent false))
          (Transformation|AttachComponentToComponent _returnvalue_21 _returnvalue_20 "Text" "KeepRelative" "KeepRelative" "KeepRelative" true)
          (Rendering|Components|TextRender|SetText _returnvalue_21 (Variables|Name|GetName))
          (Rendering|Components|TextRender|SetTextRenderColor _returnvalue_21 (Math|Conversions|ToColor(LinearColor) (Variables|Name|GetText%20Color) false)))))))

(fn AddFences
  (params (InputPin :type Spline%20Mesh%20Component%20Object%20Reference))
  (bind _returnvalue (Transformation|GetSocketLocation InputPin "FenceA"))
  (bind _returnvalue_2 (Transformation|GetSocketLocation InputPin "FenceC"))
  (bind _returnvalue_3 (Transformation|GetSocketLocation InputPin "FenceB"))
  (bind _fence_instanced_mesh (Variables|Default|GetFence%20Instanced%20Mesh))
  (Class|InstancedStaticMeshComponent|AddInstanceWorldSpace _fence_instanced_mesh (Math|Transform|MakeTransform _returnvalue (Math|Rotator|FindLookatRotation _returnvalue _returnvalue_2) (Math|Vector|MakeVector (/ (Math|Vector|VectorLength (- _returnvalue _returnvalue_2)) 1e+03) 1.0 1.0)))
  (Class|InstancedStaticMeshComponent|AddInstanceWorldSpace _fence_instanced_mesh (Math|Transform|MakeTransform _returnvalue_3 (Math|Rotator|FindLookatRotation _returnvalue_3 _returnvalue_2) (Math|Vector|MakeVector (/ (Math|Vector|VectorLength (- _returnvalue_2 _returnvalue_3)) 1e+03) 1.0 1.0))))

(fn AddSteps
  (params (Opposite%20Side :type Boolean) (Platform%20End%20B :type Boolean))
  (bind _returnvalue (Math|Float|SelectFloat -1.0 1.0 Opposite%20Side))
  (bind _returnvalue_2 (Math|Float|SelectFloat -1.0 1.0 Platform%20End%20B))
  (bind _tiles_color (Variables|Platform|GetTiles%20Color))
  (bind _spline (Variables|Default|GetSpline))
  (bind _position (Variables|Default|GetPosition))
  (bind _resulting_length (Variables|Default|GetResulting%20Length))
  (bind _doubletrack (Variables|Default|GetDoubleTrack))
  (bind _tiles_grunge_contrast (Variables|Platform|GetTiles%20Grunge%20Contrast))
  (bind _double_track_spacing (Variables|Default|GetDouble%20Track%20Spacing))
  (bind _defaultsceneroot (Variables|Default|GetDefaultSceneRoot))
  (bind _rail_top_height (Variables|Default|GetRail%20Top%20Height))
  (bind _returnvalue_3 (Math|Conversions|ToLinearColor(Color) _tiles_color))
  (bind _returnvalue_4 (/ _resulting_length 2.0))
  (bind _returnvalue_5 (Transformation|GetWorldLocation _defaultsceneroot))
  (bind _returnvalue_6 (and _doubletrack Opposite%20Side))
  (bind _returnvalue_7 (Math|Conversions|ToVector(LinearColor) _returnvalue_3))
  (bind _returnvalue_8 (Math|Conversions|ToFloat(Boolean) _returnvalue_6))
  (bind _returnvalue_9 (- _position _returnvalue_4))
  (bind _returnvalue_10 (+ _position _returnvalue_4))
  (bind _returnvalue_11 (* _double_track_spacing _returnvalue_8))
  (bind _returnvalue_12 (select Platform%20End%20B _returnvalue_10 _returnvalue_9))
  (bind _returnvalue_13 (Spline|GetDirectionatDistanceAlongSpline _spline _returnvalue_12 "World"))
  (bind _returnvalue_14 (Spline|GetLocationatDistanceAlongSpline _spline _returnvalue_12 "World"))
  (bind _returnvalue_15 (Class|SplineComponent|GetRightVectoratDistanceAlongSpline _spline _returnvalue_12 "World"))
  (bind _returnvalue_16 (Math|Conversions|RotationFromXVector _returnvalue_13))
  (bind _returnvalue_17 (- _returnvalue_14 _returnvalue_5))
  (bind _returnvalue_18 (+ _returnvalue_17 (Math|Vector|MakeVector 0.0 0.0 _rail_top_height)))
  (bind _returnvalue_19 (AddComponent|AddStaticMeshComponent false (Math|Transform|MakeTransform (- _returnvalue_18 (* _returnvalue_15 (+ _returnvalue_11 (* (Variables|Platform|GetAdjust%20Lateral%20Position) (select Opposite%20Side 1.0 -1.0))))) _returnvalue_16 (Math|Vector|MakeVector _returnvalue_2 _returnvalue 1.0))))
  ;[1 1 1] Pedestrian Crossing
  (if (Variables|Platform|GetPedestrian%20Crossing)
    (bind _returnvalue_20 (AddComponent|AddStaticMeshComponent false (Math|Transform|MakeTransform (- _returnvalue_18 (* _returnvalue_15 _returnvalue_11)) _returnvalue_16 (Math|Vector|MakeVector _returnvalue_2 _returnvalue 1.0))))
    (Rendering|Material|SetVectorParameterValueonMaterials _returnvalue_20 "TilesColor" _returnvalue_7)
    (Rendering|Material|SetScalarParameterValueonMaterials _returnvalue_20 "Grunge Contrast" _tiles_grunge_contrast))
  (Rendering|Material|SetVectorParameterValueonMaterials _returnvalue_19 "TilesColor" _returnvalue_7)
  (Rendering|Material|SetVectorParameterValueonMaterials _returnvalue_19 "MetalColor" (Math|Conversions|ToVector(LinearColor) (Math|Conversions|ToLinearColor(Color) (Variables|AdditionalMeshes|GetFence%20Color))))
  (Rendering|Material|SetScalarParameterValueonMaterials _returnvalue_19 "Grunge Contrast" _tiles_grunge_contrast))