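; BP_Track is a railway track actor built in the construction script from an editable spline, optionally double, closed-loop or electrified.
; For double or terrain-aligned track it resamples the spline into derived splines, using line traces for terrain and saved points when no terrain is hit.
; These feed spline-mesh rails, instanced catenary and dead ends, and can reposition linked BP_Trains.
; DeformLandscape instead fits the landscape to the original spline.
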(event EventBeginPlay)

(event Collision|EventActorBeginOverlap
  (params (OtherActor :type Actor%20Object%20Reference)))

(event EventTick
  (params (DeltaSeconds :type Float%20%28single-precision%29)))

(fn ConstructionScript
  (bind _splinesecondtrack (Variables|Default|GetSplineSecondTrack))
  (bind _spine2_points (Variables|AlignToTerrain|GetSpine2%20Points))
  (bind _spine2_points_2 (Variables|AlignToTerrain|GetSpine2%20Points))
  (bind _spinesecond_points (Variables|AlignToTerrain|GetSpineSecond%20Points))
  (bind _splinesecondtrack_2 (Variables|Default|GetSplineSecondTrack))
  (bind _spinesecond_points_2 (Variables|AlignToTerrain|GetSpineSecond%20Points))
  (bind _splinesecondtrack_3 (Variables|Default|GetSplineSecondTrack))
  (Utilities|FlowControl|Sequence
    (:then_0
      (Spline|SetClosedLoop (Variables|Default|GetSpline) (Variables|TrackConfiguration|GetClosed%20Loop) true)
      (Transformation|SetActorRotation "0, 0, 0")
      (Transformation|SetActorScale3D "1.000000,1.000000,1.000000")
      (Variables|AligntoTerrain|SetUpdate false))
    (:then_1
      ;[1 1 1] Align to Terrain
      (if (or (Variables|TrackConfiguration|GetDouble%20Track) (Variables|AligntoTerrain|GetAlign%20to%20Terrain))
        (CallFunction|SetTrackSplines)
        (Variables|Default|SetSpline_Current (Variables|Default|GetSpline2))
        (else
          (Variables|Default|SetSpline_Current (Variables|Default|GetSpline)))))
    (:then_2
      ;[1 1 1] Check whether terrain aligning failed due to Landscape not yet loaded
      (if (Variables|AligntoTerrain|GetAlign%20to%20Terrain)
        (if (== (Variables|AlignToTerrain|GetTerrain%20Hits%20count) 0)
          ;[1 1 1] Recover Splines from saved points
          (Utilities|FlowControl|Sequence
            (:then_0
              (Spline|ClearSplinePoints (Variables|Default|GetSpline_Current) true)
              (for _index (range 0 (- (Utilities|Array|Length _spine2_points_2) 1))
                (Spline|AddSplinePoint (Variables|Default|GetSpline_Current) (Utilities|Array|Get(acopy) _spine2_points_2 _index) "Local" true)))
            (:then_1
              (if (Variables|TrackConfiguration|GetDouble%20Track)
                (Spline|ClearSplinePoints _splinesecondtrack_3 true)
                (for _index_2 (range 0 (- (Utilities|Array|Length _spinesecond_points_2) 1))
                  (Spline|AddSplinePoint _splinesecondtrack_3 (Utilities|Array|Get(acopy) _spinesecond_points_2 _index_2) "Local" true)))))
          (else
            ;[1 1 1] Save backup points arrays so Splines can be restored later
            (Utilities|FlowControl|Sequence
              (:then_0
                (Utilities|Array|Clear _spine2_points)
                (for _index_3 (range 0 (- (Spline|GetNumberOfSplinePoints (Variables|Default|GetSpline_Current)) 1))
                  (Utilities|Array|Add _spine2_points (Spline|GetLocationatSplinePoint (Variables|Default|GetSpline_Current) _index_3 "Local"))))
              (:then_1
                (if (Variables|TrackConfiguration|GetDouble%20Track)
                  (Utilities|Array|Clear _spinesecond_points)
                  (for _index_4 (range 0 (- (Spline|GetNumberOfSplinePoints _splinesecondtrack_2) 1))
                    (Utilities|Array|Add _spinesecond_points (Spline|GetLocationatSplinePoint _splinesecondtrack_2 _index_4 "Local"))))))))))
    (:then_4
      (Utilities|FlowControl|Sequence
        (:then_0
          ;[1 1 1] Add Track Spline Meshes
          (CallFunction|AddTrackSplineMeshes (Variables|Default|GetSpline_Current) false)
          (if (Variables|TrackConfiguration|GetDouble%20Track)
            (CallFunction|AddTrackSplineMeshes (Variables|Default|GetSplineSecondTrack) true)))
        (:then_1
          ;[1 1 1] Get Track Length
          (Variables|TrackConfiguration|SetTrack%20Length%20%28m%29 (/ (Spline|GetSplineLength (Variables|Default|GetSpline_Current)) 1e+02)))
        (:then_2
          ;[1 1 1] Update all Trains connected to this Track
          (if (Variables|TrackConfiguration|GetAuto%20Update%20Trains%20on%20this%20Track)
            (bind _outactors (Actor|GetAllActorsOfClass "/Game/Railway_System/Blueprints/BP_Train.BP_Train_C"))
            (for _array_element _outactors
              (if (== (Variables|/Game/Railway_System/Blueprints/BP_Train.BP_Train_C|GetTrack%20Pick _array_element) self)
                (Default|SearchNearestTrack _array_element)
                (Default|PositionBogiesandCars _array_element)))))
        (:then_3
          ;[1 1 1] Dead Ends
          (if (not (Variables|TrackConfiguration|GetClosed%20Loop))
            (CallFunction|AddDeadEnd false (Variables|Default|GetSpline_Current) (Variables|TrackConfiguration|GetDead%20End%20%28Start%29))
            (CallFunction|AddDeadEnd true (Variables|Default|GetSpline_Current) (Variables|TrackConfiguration|GetDead%20End%20%28End%29))
            (if (Variables|TrackConfiguration|GetDouble%20Track)
              (CallFunction|AddDeadEnd false _splinesecondtrack (Variables|TrackConfiguration|GetDead%20End%20%28End%29))
              (CallFunction|AddDeadEnd true _splinesecondtrack (Variables|TrackConfiguration|GetDead%20End%20%28Start%29)))))))))

(fn SetTrackSplines
  (bind _spline (Variables|Default|GetSpline))
  (bind _actors_to_ignore_final (LocalVariables|GetActors%20to%20Ignore%20final))
  (bind _terraintrace_distance__m_ (Variables|AligntoTerrain|GetTerrainTrace%20Distance%20%28m%29))
  (bind _spline_2 (Variables|Default|GetSpline))
  (bind _returnvalue (Spline|GetSplineLength _spline_2))
  (bind _returnvalue_2 (Spline|GetSplineLength _spline))
  (bind _returnvalue_3 (* _terraintrace_distance__m_ 1e+02))
  (bind _returnvalue_4 (/ _returnvalue_2 _returnvalue_3))
  (bind _returnvalue_5 (Math|Float|Truncate _returnvalue_4))
  (bind _returnvalue_6 (Math|Integer|Clamp(Integer) _returnvalue_5 1 10000))
  (Utilities|FlowControl|Sequence
    (:then_0
      ;[1 1 1] Add new Spline2
      (bind _returnvalue_7 (AddComponent|AddSplineComponent false))
      (bind _output_get (Variables|Default|SetSpline2 _returnvalue_7))
      (Spline|ClearSplinePoints _output_get false)
      (Spline|SetClosedLoop _output_get (Variables|TrackConfiguration|GetClosed%20Loop) false))
    (:then_1
      (if (Variables|TrackConfiguration|GetDouble%20Track)
        ;[1 1 1] Add new Spline Second Track
        (bind _returnvalue_8 (AddComponent|AddSplineComponent false))
        (bind _output_get_2 (Variables|Default|SetSplineSecondTrack _returnvalue_8))
        (Spline|ClearSplinePoints _output_get_2 false)
        (Spline|SetClosedLoop _output_get_2 (Variables|TrackConfiguration|GetClosed%20Loop) false)))
    (:then_2
      ;[1 1 1] Actors to ignore
      (if (Variables|AligntoTerrain|GetAlign%20to%20Terrain)
        (Utilities|Array|Clear _actors_to_ignore_final)
        (bind _outactors (Actor|GetAllActorsOfClass "/Game/Railway_System/Blueprints/BP_Tunnel.BP_Tunnel_C"))
        (Utilities|Array|AppendArray _actors_to_ignore_final _outactors)
        (bind _outactors_2 (Actor|GetAllActorsOfClass "/Game/Railway_System/Blueprints/BP_Crossing.BP_Crossing_C"))
        (Utilities|Array|AppendArray _actors_to_ignore_final _outactors_2)
        (bind _outactors_3 (Actor|GetAllActorsOfClass "BP_Track_C"))
        (Utilities|Array|AppendArray _actors_to_ignore_final _outactors_3)
        (bind _outactors_4 (Actor|GetAllActorsOfClass "/Game/Railway_System/Blueprints/BP_Train.BP_Train_C"))
        (Utilities|Array|AppendArray _actors_to_ignore_final _outactors_4)
        (bind _outactors_5 (Actor|GetAllActorsOfClass "/Game/Railway_System/Blueprints/BP_Platform.BP_Platform_C"))
        (Utilities|Array|AppendArray _actors_to_ignore_final _outactors_5)
        (Utilities|Array|AppendArray _actors_to_ignore_final (Variables|AlignToTerrain|GetActors%20to%20Ignore))))
    (:then_3
      (Utilities|FlowControl|Sequence
        (:then_0
          (Variables|AlignToTerrain|SetTerrain%20Hits%20count 0 :!label _label)
          (for _index (range 0 (select (Variables|TrackConfiguration|GetClosed%20Loop) (- _returnvalue_6 1) _returnvalue_6))
            (if (Variables|AligntoTerrain|GetAlign%20to%20Terrain)
              ;[1 1 1] Align to Terrain
              (bind (_outhit _returnvalue_9) (Collision|LineTraceForObjects (+ (select (Variables|TrackConfiguration|GetDouble%20Track) (+ (Spline|GetLocationatDistanceAlongSpline _spline_2 (Math|Float|SelectFloat (- _returnvalue (* _index (/ _returnvalue (Math|Conversions|ToFloat(Integer) _returnvalue_6)))) (* _index (/ _returnvalue (Math|Conversions|ToFloat(Integer) _returnvalue_6))) (LocalVariables|GetSecondTrack)) "World") (* (Class|SplineComponent|GetRightVectoratDistanceAlongSpline _spline_2 (Math|Float|SelectFloat (- _returnvalue (* _index (/ _returnvalue (Math|Conversions|ToFloat(Integer) _returnvalue_6)))) (* _index (/ _returnvalue (Math|Conversions|ToFloat(Integer) _returnvalue_6))) (LocalVariables|GetSecondTrack)) "World") (* (/ (Variables|TrackConfiguration|GetDoubleTrack%20Spacing) 2.0) (Math|Float|SelectFloat -1.0 1.0 (LocalVariables|GetSecondTrack))))) (Spline|GetLocationatDistanceAlongSpline _spline_2 (Math|Float|SelectFloat (- _returnvalue (* _index (/ _returnvalue (Math|Conversions|ToFloat(Integer) _returnvalue_6)))) (* _index (/ _returnvalue (Math|Conversions|ToFloat(Integer) _returnvalue_6))) (LocalVariables|GetSecondTrack)) "World")) (Math|Vector|MakeVector 0.0 0.0 (Variables|AligntoTerrain|GetTerrainTraceHeight%20up))) (- (select (Variables|TrackConfiguration|GetDouble%20Track) (+ (Spline|GetLocationatDistanceAlongSpline _spline_2 (Math|Float|SelectFloat (- _returnvalue (* _index (/ _returnvalue (Math|Conversions|ToFloat(Integer) _returnvalue_6)))) (* _index (/ _returnvalue (Math|Conversions|ToFloat(Integer) _returnvalue_6))) (LocalVariables|GetSecondTrack)) "World") (* (Class|SplineComponent|GetRightVectoratDistanceAlongSpline _spline_2 (Math|Float|SelectFloat (- _returnvalue (* _index (/ _returnvalue (Math|Conversions|ToFloat(Integer) _returnvalue_6)))) (* _index (/ _returnvalue (Math|Conversions|ToFloat(Integer) _returnvalue_6))) (LocalVariables|GetSecondTrack)) "World") (* (/ (Variables|TrackConfiguration|GetDoubleTrack%20Spacing) 2.0) (Math|Float|SelectFloat -1.0 1.0 (LocalVariables|GetSecondTrack))))) (Spline|GetLocationatDistanceAlongSpline _spline_2 (Math|Float|SelectFloat (- _returnvalue (* _index (/ _returnvalue (Math|Conversions|ToFloat(Integer) _returnvalue_6)))) (* _index (/ _returnvalue (Math|Conversions|ToFloat(Integer) _returnvalue_6))) (LocalVariables|GetSecondTrack)) "World")) (Math|Vector|MakeVector 0.0 0.0 (Variables|AligntoTerrain|GetTerrainTraceHeight%20down))) (Variables|AligntoTerrain|GetTerrain%20ObjectTypes) false (LocalVariables|GetActors%20to%20Ignore%20final) "None"))
              (if _returnvalue_9
                (Math|Integer|IncrementInt (Variables|AlignToTerrain|GetTerrain%20Hits%20count)
                  (:%20%20
                    (Spline|AddSplinePoint (select (LocalVariables|GetSecondTrack) (Variables|Default|GetSplineSecondTrack) (Variables|Default|GetSpline2)) (select (Variables|AligntoTerrain|GetAlign%20to%20Terrain) (.location _outhit) (select (Variables|TrackConfiguration|GetDouble%20Track) (+ (Spline|GetLocationatDistanceAlongSpline _spline_2 (Math|Float|SelectFloat (- _returnvalue (* _index (/ _returnvalue (Math|Conversions|ToFloat(Integer) _returnvalue_6)))) (* _index (/ _returnvalue (Math|Conversions|ToFloat(Integer) _returnvalue_6))) (LocalVariables|GetSecondTrack)) "World") (* (Class|SplineComponent|GetRightVectoratDistanceAlongSpline _spline_2 (Math|Float|SelectFloat (- _returnvalue (* _index (/ _returnvalue (Math|Conversions|ToFloat(Integer) _returnvalue_6)))) (* _index (/ _returnvalue (Math|Conversions|ToFloat(Integer) _returnvalue_6))) (LocalVariables|GetSecondTrack)) "World") (* (/ (Variables|TrackConfiguration|GetDoubleTrack%20Spacing) 2.0) (Math|Float|SelectFloat -1.0 1.0 (LocalVariables|GetSecondTrack))))) (Spline|GetLocationatDistanceAlongSpline _spline_2 (Math|Float|SelectFloat (- _returnvalue (* _index (/ _returnvalue (Math|Conversions|ToFloat(Integer) _returnvalue_6)))) (* _index (/ _returnvalue (Math|Conversions|ToFloat(Integer) _returnvalue_6))) (LocalVariables|GetSecondTrack)) "World"))) "World" true :!label _label_2)))
                (else
                  (Spline|AddSplinePoint (select (LocalVariables|GetSecondTrack) (Variables|Default|GetSplineSecondTrack) (Variables|Default|GetSpline2)) (select (Variables|TrackConfiguration|GetDouble%20Track) (+ (Spline|GetLocationatDistanceAlongSpline _spline_2 (Math|Float|SelectFloat (- _returnvalue (* _index (/ _returnvalue (Math|Conversions|ToFloat(Integer) _returnvalue_6)))) (* _index (/ _returnvalue (Math|Conversions|ToFloat(Integer) _returnvalue_6))) (LocalVariables|GetSecondTrack)) "World") (* (Class|SplineComponent|GetRightVectoratDistanceAlongSpline _spline_2 (Math|Float|SelectFloat (- _returnvalue (* _index (/ _returnvalue (Math|Conversions|ToFloat(Integer) _returnvalue_6)))) (* _index (/ _returnvalue (Math|Conversions|ToFloat(Integer) _returnvalue_6))) (LocalVariables|GetSecondTrack)) "World") (* (/ (Variables|TrackConfiguration|GetDoubleTrack%20Spacing) 2.0) (Math|Float|SelectFloat -1.0 1.0 (LocalVariables|GetSecondTrack))))) (Spline|GetLocationatDistanceAlongSpline _spline_2 (Math|Float|SelectFloat (- _returnvalue (* _index (/ _returnvalue (Math|Conversions|ToFloat(Integer) _returnvalue_6)))) (* _index (/ _returnvalue (Math|Conversions|ToFloat(Integer) _returnvalue_6))) (LocalVariables|GetSecondTrack)) "World")) "World" true)))
              (else
                (goto _label_2)))))
        (:then_1
          (if (Variables|TrackConfiguration|GetDouble%20Track)
            (LocalVariables|SetSecondTrack true)
            (goto _label)))))))

(fn AddTrackSplineMeshes
  (params (Spline :type Spline%20Component%20Object%20Reference) (SecondTrack :type Boolean))
  (bind _returnvalue (Spline|GetSplineLength Spline))
  (bind _returnvalue_2 (Spline|GetSplineLength Spline))
  (bind _rail_top_height (Variables|TrackConfiguration|GetRail%20Top%20Height))
  (bind _mesh_length (Variables|TrackConfiguration|GetMesh%20Length))
  (bind _mesh_length_2 (Variables|TrackConfiguration|GetMesh%20Length))
  (bind _returnvalue_3 (Math|Vector|MakeVector 0.0 0.0 _rail_top_height))
  (bind _returnvalue_4 (/ _returnvalue_2 _mesh_length))
  (bind _returnvalue_5 (- _returnvalue 0.1))
  (bind _returnvalue_6 (Math|Float|Truncate _returnvalue_4))
  (bind _returnvalue_7 (Math|Integer|Clamp(Integer) _returnvalue_6 1 10000))
  (bind _returnvalue_8 (Math|Conversions|ToFloat(Integer) _returnvalue_7))
  (bind _returnvalue_9 (/ _returnvalue_5 _returnvalue_8))
  (if (not (Variables|TrackConfiguration|GetSpline%20Editing%20Mode))
    (Utilities|FlowControl|Sequence
      (:then_0
        (for _index (range 0 (- _returnvalue_7 1))
          (bind _returnvalue_10 (AddComponent|AddSplineMeshComponent false))
          (SplineMesh|SetStartandEnd _returnvalue_10 (+ (Spline|GetLocationatDistanceAlongSpline Spline (* _index _returnvalue_9) "Local") _returnvalue_3) (* (Math|Vector|Normalize (Spline|GetTangentatDistanceAlongSpline Spline (* _index _returnvalue_9) "Local")) _mesh_length_2) (+ (Spline|GetLocationatDistanceAlongSpline Spline (* (+ _index 1) _returnvalue_9) "Local") _returnvalue_3) (* (Math|Vector|Normalize (Spline|GetTangentatDistanceAlongSpline Spline (* (+ _index 1) _returnvalue_9) "Local")) _mesh_length_2) true :!class /Script/Engine.SplineMeshComponent)
          (Rendering|Material|SetScalarParameterValueonMaterials _returnvalue_10 "Dirtiness" (Variables|TrackAppearance|GetDirtiness))
          (Rendering|Material|SetVectorParameterValueonMaterials _returnvalue_10 "Tint" (Math|Conversions|ToVector(LinearColor) (Math|Conversions|ToLinearColor(Color) (Variables|TrackAppearance|GetGravel%20Tint))))
          (if (Variables|TrackAppearance|GetWooden%20Track)
            (Components|StaticMesh|SetStaticMesh _returnvalue_10 "/Game/Railway_System/Meshes/Track/SM_Track_Wooden.SM_Track_Wooden"))))
      (:then_1
        (CallFunction|AddElectrification Spline SecondTrack)))))

(fn AddElectrification
  (params (Spline :type Spline%20Component%20Object%20Reference) (Second%20Track :type Boolean))
  (bind _returnvalue (Spline|GetSplineLength Spline))
  (bind _mast_spacing__m_ (Variables|Electrification|GetMast%20Spacing%20%28m%29))
  (bind _returnvalue_2 (* _mast_spacing__m_ 1e+02))
  (bind _returnvalue_3 (/ _returnvalue _returnvalue_2))
  (bind _returnvalue_4 (Math|Float|Truncate _returnvalue_3))
  (bind _returnvalue_5 (+ _returnvalue_4 1))
  (if (Variables|Electrification|GetElectrified%20Track)
    ;[1 1 1] Prepare Instanced Static Mesh Components
    (bind _returnvalue_6 (AddComponent|AddInstancedStaticMeshComponent false))
    (bind _returnvalue_7 (AddComponent|AddInstancedStaticMeshComponent false))
    (Rendering|Material|SetScalarParameterValueonMaterials _returnvalue_6 "Dirtiness" (Variables|TrackAppearance|GetDirtiness))
    (for _index (range 0 _returnvalue_5)
      (Components|InstancedStaticMesh|AddInstance _returnvalue_6 (Math|Transform|MakeTransform (+ (Spline|GetLocationatDistanceAlongSpline Spline (* _index (/ _returnvalue (Math|Conversions|ToFloat(Integer) _returnvalue_5))) "Local") (Math|Vector|MakeVector 0.0 0.0 (Variables|TrackConfiguration|GetRail%20Top%20Height))) (Spline|GetRotationatDistanceAlongSpline Spline (* _index (/ _returnvalue (Math|Conversions|ToFloat(Integer) _returnvalue_5))) "Local") "1,1,1"))
      (if (== _index 0)
        _
        (else
          (Components|InstancedStaticMesh|AddInstance _returnvalue_7 (Math|Transform|MakeTransform (+ (Spline|GetLocationatDistanceAlongSpline Spline (* _index (/ _returnvalue (Math|Conversions|ToFloat(Integer) _returnvalue_5))) "Local") (Math|Vector|MakeVector 0.0 0.0 (Variables|TrackConfiguration|GetRail%20Top%20Height))) (Math|Rotator|FindLookatRotation (LocalVariables|GetPrevious%20Location) (+ (Spline|GetLocationatDistanceAlongSpline Spline (* _index (/ _returnvalue (Math|Conversions|ToFloat(Integer) _returnvalue_5))) "Local") (Math|Vector|MakeVector 0.0 0.0 (Variables|TrackConfiguration|GetRail%20Top%20Height)))) (Math|Vector|MakeVector (/ (Math|Vector|Distance(Vector) (+ (Spline|GetLocationatDistanceAlongSpline Spline (* _index (/ _returnvalue (Math|Conversions|ToFloat(Integer) _returnvalue_5))) "Local") (Math|Vector|MakeVector 0.0 0.0 (Variables|TrackConfiguration|GetRail%20Top%20Height))) (LocalVariables|GetPrevious%20Location)) 5e+03) 1.0 1.0)))))
      (LocalVariables|SetPrevious%20Location (+ (Spline|GetLocationatDistanceAlongSpline Spline (* _index (/ _returnvalue (Math|Conversions|ToFloat(Integer) _returnvalue_5))) "Local") (Math|Vector|MakeVector 0.0 0.0 (Variables|TrackConfiguration|GetRail%20Top%20Height)))))))

(fn AddDeadEnd
  (params (TrackEnd :type Boolean) (Spline :type Spline%20Component%20Object%20Reference) (Add%20Mesh :type Boolean))
  (bind _returnvalue (Spline|GetSplineLength Spline))
  (bind _returnvalue_2 (- _returnvalue 2.0))
  (bind _returnvalue_3 (Math|Float|SelectFloat _returnvalue_2 0.0 TrackEnd))
  (if (and Add%20Mesh (not (Variables|TrackConfiguration|GetSpline%20Editing%20Mode)))
    (AddComponent|AddStaticMeshComponent false (Math|Transform|MakeTransform (+ (- (Spline|GetLocationatDistanceAlongSpline Spline _returnvalue_3 "World") (Transformation|GetWorldLocation (Variables|Default|GetSpline))) (Math|Vector|MakeVector 0.0 0.0 (Variables|TrackConfiguration|GetRail%20Top%20Height))) (Math|Conversions|RotationFromXVector (* (Spline|GetDirectionatDistanceAlongSpline Spline _returnvalue_3 "World") (Math|Float|SelectFloat -1.0 1.0 TrackEnd))) "1,1,1"))))

(fn DeformLandscape
  (bind _double_track (Variables|TrackConfiguration|GetDouble%20Track))
  (bind _doubletrack_spacing (Variables|TrackConfiguration|GetDoubleTrack%20Spacing))
  (bind _spline_width_adjust__m_ (Variables|DeformLandscape|GetSpline%20Width%20Adjust%20%28m%29))
  (bind _side_falloff__m_ (Variables|DeformLandscape|GetSide%20Falloff%20%28m%29))
  (bind _returnvalue (+ _doubletrack_spacing 2.5e+02))
  (bind _returnvalue_2 (* _spline_width_adjust__m_ 1e+02))
  (bind _returnvalue_3 (* _side_falloff__m_ 1e+02))
  (bind _returnvalue_4 (Math|Float|SelectFloat _returnvalue 3.5e+02 _double_track))
  (bind _returnvalue_5 (+ _returnvalue_4 _returnvalue_2))
  ;[1 1 1] Check if Landscape shoud be deformed
  (Utilities|IsValid (Variables|DeformLandscape|GetLandscape%20to%20deform)
    (:Is%20Valid
      (if (Variables|AligntoTerrain|GetAlign%20to%20Terrain)
        (Development|PrintString "Disable Align to Terrain" true true "(R=0.014235,G=0.072334,B=0.166667,A=1.000000)" 5.0)
        (else
          (Landscape|Editor|EditorApplySpline (Variables|DeformLandscape|GetLandscape%20to%20deform) (Variables|Default|GetSpline) _returnvalue_5 _returnvalue_5 _returnvalue_3 _returnvalue_3 0.0 0.0 5 (Variables|DeformLandscape|GetRaise%20Heights) (Variables|DeformLandscape|GetLower%20Heights) 0))))
    (:Is%20Not%20Valid
      (Development|PrintString "Pick Landscape to Deform" true true "(R=0.014235,G=0.072334,B=0.166667,A=1.000000)" 5.0))))