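; Blueprint function library for the railway system that locates the track and spline position nearest to a world location.
; The distance search samples a spline at fixed segment steps given in meters and returns the closest sample's distance along the spline and its distance to the location.
; The track search runs that search on every BP_Track actor's current spline and picks the closest, flagging whether any track exists.
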(fn SearchNearestDistanceonSpline
  (params (Spline :type Spline%20Component%20Object%20Reference) (Location :type Vector) (Spline%20Segment%20Length%20%28m%29 :type Float%20%28single-precision%29))
  (bind _returnvalue (* Spline%20Segment%20Length%20%28m%29 1e+02))
  (LocalVariables|SetSegmentLength _returnvalue)
  (LocalVariables|SetMinDistance (Math|Vector|VectorLength (- Location (Spline|GetLocationatDistanceAlongSpline Spline 0.0 "World"))))
  (for _index (range 1 (Math|Float|Truncate (/ (Spline|GetSplineLength Spline) _returnvalue)))
    (if (< (Math|Vector|VectorLength (- Location (Spline|GetLocationatDistanceAlongSpline Spline (* _index (LocalVariables|GetSegmentLength)) "World"))) (LocalVariables|GetMinDistance))
      (LocalVariables|SetMinDistance (Math|Vector|VectorLength (- Location (Spline|GetLocationatDistanceAlongSpline Spline (* _index (LocalVariables|GetSegmentLength)) "World"))))
      (LocalVariables|SetPositition%20Index _index)))
  (return (* (LocalVariables|GetPositition%20Index) (LocalVariables|GetSegmentLength)) (LocalVariables|GetMinDistance)))

(fn SearchNearestBPTrack
  (params (Location :type Vector))
  (bind _outactors (Actor|GetAllActorsOfClass 0 "/Game/Railway_System/Blueprints/BP_Track.BP_Track_C"))
  (if (== (Utilities|Array|Length _outactors) 0)
    (LocalVariables|SetTrackSelected false)
    (else
      (LocalVariables|SetTrackSelected true)
      (for (_array_element _array_index) _outactors
        (bind _min_distance_to_location_ (CallFunction|SearchNearestDistanceonSpline (Variables|/Game/Railway_System/Blueprints/BP_Track.BP_Track_C|GetSpline_Current _array_element) Location 1e+01))
        (if (or (< _min_distance_to_location_ (LocalVariables|GetMinDistance)) (== _array_index 0))
          (LocalVariables|SetMinDistance _min_distance_to_location_)
          (LocalVariables|SetTrack _array_index)))
      (return (LocalVariables|GetTrackSelected) (Utilities|Array|Get(acopy) _outactors (LocalVariables|GetTrack))))))